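; An actor Blueprint that visualizes AR-tracked QR codes with debug drawing, driven by ARTrackableNotify component events.
; The add event only prints a message, while the update event continues only for geometry that casts to ARTrackedQRCode.
; It transforms half the code's estimated size into world space, then draws the decoded text and an oriented box there for a few seconds, followed by a debug print.
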(event OnAddTrackedGeometry(ARTrackableNotify)
  (params (TrackedGeometry :type AR%20Tracked%20Geometry%20Object%20Reference))
  (Development|PrintString "Add Tracked Geomentry Turned on" true true "(R=0.034897,G=0.077698,B=1.000000,A=1.000000)" 5e+01))

(event OnUpdateTrackedGeometry(ARTrackableNotify)
  (params (TrackedGeometry :type AR%20Tracked%20Geometry%20Object%20Reference))
  (bind _asartracked_qrcode (Utilities|Casting|CastToARTrackedQRCode TrackedGeometry))
  (Rendering|Debug|DrawDebugString (Math|Transform|TransformLocation (Class|ARTrackedGeometry|GetLocaltoWorldTransform _asartracked_qrcode) (/ (Math|Vector|MakeVector 0.0 (.X (Math|Vector2D|BreakVector2D (Class|ARTrackedImage|GetEstimateSize _asartracked_qrcode))) (.Y (Math|Vector2D|BreakVector2D (Class|ARTrackedImage|GetEstimateSize _asartracked_qrcode)))) 2.0)) (Variables|/Script/AugmentedReality.ARTrackedQRCode|GetQRCode _asartracked_qrcode) 0 "(R=1.000000,G=1.000000,B=1.000000,A=1.000000)" 3.0)
  (Rendering|Debug|DrawDebugBox (Math|Transform|TransformLocation (Class|ARTrackedGeometry|GetLocaltoWorldTransform _asartracked_qrcode) (/ (Math|Vector|MakeVector 0.0 (.X (Math|Vector2D|BreakVector2D (Class|ARTrackedImage|GetEstimateSize _asartracked_qrcode))) (.Y (Math|Vector2D|BreakVector2D (Class|ARTrackedImage|GetEstimateSize _asartracked_qrcode)))) 2.0)) (/ (Math|Vector|MakeVector 0.0 (.X (Math|Vector2D|BreakVector2D (Class|ARTrackedImage|GetEstimateSize _asartracked_qrcode))) (.Y (Math|Vector2D|BreakVector2D (Class|ARTrackedImage|GetEstimateSize _asartracked_qrcode)))) 2.0) "(R=0.000000,G=1.000000,B=0.119931,A=1.000000)" (Math|Transform|TransformRotation (Class|ARTrackedGeometry|GetLocaltoWorldTransform _asartracked_qrcode) "0, 0, 0") 3.0 5e+01)
  (Development|PrintString "Got to the end....." true true "(R=0.000000,G=0.660000,B=1.000000,A=1.000000)" 1e+01))

(fn ConstructionScript)